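; BP_MoveLeftRight is an actor that slides its static mesh back and forth along relative X while a BP_MyBox overlap is active.
; On BeginPlay it binds to the begin and end overlap dispatchers of every BP_MyBox in the level to start and stop the motion.
; A Timeline drives the offset, flipping IsMoveRight on finish to alternate play and reverse in an endless ping-pong until stopped.
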(event EventPlay
  (if (Variables|Default|GetIsMoveRight) :!label _label
    (bind _value (Timeline|타임라인_0 Play)
      (:Update
        (Transformation|SetRelativeLocation (Variables|Default|GetStaticMesh) (Math|Vector|MakeVector (* _value 1e+03) 0.0 0.0) false false))
      (:Finished
        (Variables|Default|SetIsMoveRight (not (Variables|Default|GetIsMoveRight)))
        (goto _label)))
    (else
      (Timeline|타임라인_0 Reverse))))

(event EventBeginPlay
  (bind _outactors (Actor|GetAllActorsOfClass "/Game/Collision/Blueprints/BP_MyBox.BP_MyBox_C"))
  (for _array_element _outactors
    (EventDispatchers|BindEventtoEventDispatcherBeginOverlap _array_element (EventDispatchers|CreateEvent :!event EventBeginOverlap))
    (EventDispatchers|BindEventtoEventDispatcherEndOverlap _array_element (EventDispatchers|CreateEvent :!event EventEndOverlap))))

(event EventStop
  (bind _value (Timeline|타임라인_0 Stop)
    (:Update
      (Transformation|SetRelativeLocation (Variables|Default|GetStaticMesh) (Math|Vector|MakeVector (* _value 1e+03) 0.0 0.0) false false))
    (:Finished
      (Variables|Default|SetIsMoveRight (not (Variables|Default|GetIsMoveRight)))
      (if (Variables|Default|GetIsMoveRight)
        (Timeline|타임라인_0 Play)
        (else
          (Timeline|타임라인_0 Reverse))))))

(fn ConstructionScript)

(fn EventBeginOverlap
  (params (bResult :type Boolean))
  (CallFunction|Play))

(fn EventEndOverlap
  (CallFunction|Stop))