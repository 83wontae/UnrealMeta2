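; Inventory component that holds item slots and shows them in a toggleable inventory widget.
; It sizes the slot array on BeginPlay, with each slot storing an item row name and a count.
; Opening creates the widget and rebuilds its list from the slots, while closing removes and clears it.
; GetItem writes a single item into the array at the default index, without searching for a free slot or refreshing the UI.
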(event EventBeginPlay
  (Utilities|Array|Resize (Variables|Default|GetInvenSlots) 10)
  (for _array_element (Variables|Default|GetInvenSlots)
    (Development|PrintString (Utilities|String|ToString(Name) (.ItemRowName (Utilities|Struct|BreakST_InvenSlot _array_element))))))

(event EventTick
  (params (DeltaSeconds :type Float%20%28single-precision%29)))

(fn OpenInven
  (Utilities|IsValid (Variables|Default|GetInventoryWidget)
    (:Is%20Not%20Valid
      (bind _returnvalue (UserInterface|CreateWidget "/Game/ShootingGame/Widget/InventoryWidget.InventoryWidget_C"))
      (bind _output_get (Variables|Default|SetInventoryWidget _returnvalue))
      (UserInterface|Viewport|AddtoViewport _output_get 0)
      (CallFunction|UpdateInventoryUI))))

(fn CloseInven
  (Utilities|IsValid (Variables|Default|GetInventoryWidget)
    (:Is%20Valid
      (Widget|RemovefromParent (Variables|Default|GetInventoryWidget))
      (Variables|Default|SetInventoryWidget 0))))

(fn ToggleInven
  (Utilities|IsValid (Variables|Default|GetInventoryWidget)
    (:Is%20Valid
      (CallFunction|CloseInven))
    (:Is%20Not%20Valid
      (CallFunction|OpenInven))))

(fn UpdateInventoryUI
  (bind _inventorywidget (Variables|Default|GetInventoryWidget))
  (Utilities|IsValid _inventorywidget
    (:Is%20Valid
      (Default|ClearList _inventorywidget)
      (for _array_element (Variables|Default|GetInvenSlots)
        (Development|PrintString (Utilities|String|ToString(Name) (.ItemRowName (Utilities|Struct|BreakST_InvenSlot _array_element))))
        (Default|AddInvenSlot (Variables|Default|GetInventoryWidget) _array_element)))))

(fn GetItem
  (params (ItemRowName :type Name))
  (Utilities|Array|SetArrayElem (Variables|Default|GetInvenSlots) 0 (Utilities|Struct|MakeST_InvenSlot ItemRowName 1)))