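; Burst weapon Blueprint for a shooting game that repeats its shooting action while the trigger is held.
; TriggerEvent starts a looping timer by function name on press and clears it on release.
; Each tick of that timer calls BurstShooting, which only plays the WeaponData shoot montage on the owning character, with no shot count limit.
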(event EventBeginPlay
  (|CallParentFunction) ; This node is disabled and will not be called.\nDrag off pins to build functionality.
)

(event Collision|EventActorBeginOverlap
  (params (OtherActor :type Actor%20Object%20Reference)))

(event EventTick
  (params (DeltaSeconds :type Float%20%28single-precision%29)))

(event EventTriggerEvent
  (params (IsPressed :type Boolean))
  (if IsPressed
    (Utilities|Time|SetTimerbyFunctionName 0 "BurstShooting" 0.2 true)
    (else
      (Utilities|Time|ClearTimerbyFunctionName 0 "BurstShooting"))))

(fn ConstructionScript
  (|CallParentFunction))

(fn BurstShooting
  (Animation|PlayAnimMontage (Variables|Default|GetOwnCharacter) (.shootmontage (Variables|Default|GetWeaponData)) 1.0 "None"))