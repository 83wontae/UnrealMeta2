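; BP_Weapon is a gun actor that plays a shoot montage on its owning character and deals hitscan damage.
; PressTrigger starts the montage, and NotifyShoot spawns a muzzle effect and plays the shot sound.
; Only when the owner is player character 0 does it call ReqShoot, which line-traces along the camera's forward vector from an offset start and applies damage to hit Characters, with debug drawing and printing left on.
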(event Custom|ReqShoot
  (params (StartPoint :type Vector) (ForwardVector :type Vector))
  (bind _outhit (Collision|LineTraceForObjects (+ StartPoint (* ForwardVector 3.5e+02)) (+ StartPoint (* ForwardVector (Variables|Default|GetDistance))) (Utilities|Array|MakeArray "ObjectTypeQuery3" "ObjectTypeQuery1" "ObjectTypeQuery2" "ObjectTypeQuery4" "ObjectTypeQuery5" "ObjectTypeQuery6") false (Utilities|Array|MakeArray (Variables|Default|GetOwnCharacter)) "Persistent"))
  (Development|PrintString (Utilities|String|Append "HitActor - " (Utilities|GetDisplayName (.HitActor (Collision|BreakHitResult _outhit)))) true true "(R=0.000000,G=0.660000,B=1.000000,A=1.000000)" 6e+01)
  (bind _ascharacter (Utilities|Casting|CastToCharacter (.HitActor (Collision|BreakHitResult _outhit))))
  (Game|Damage|ApplyDamage _ascharacter 1e+01 (Pawn|GetController (Variables|Default|GetOwnCharacter)) self))

(event EventBeginPlay
  (Audio|Components|Audio|SetSound (Variables|Default|GetAudio) (Variables|Default|GetShootSound)))

(event EventPressTrigger
  (Animation|PlayAnimMontage (Variables|Default|GetOwnCharacter) (Variables|Default|GetShootMontage) 1.0 "None"))

(event EventNotifyShoot
  (bind _returnvalue (Game|GetPlayerCameraManager 0))
  (bind _staticmesh (Variables|Default|GetStaticMesh))
  (bind _returnvalue_2 (Transformation|GetSocketTransform _staticmesh "Muzzle" "RTS_World"))
  (Effects|SpawnEmitteratLocation "/Game/StarterContent/Particles/P_Explosion.P_Explosion" (.location _returnvalue_2) (.rotation _returnvalue_2) "0.300000,0.300000,0.300000" true "AutoRelease")
  (Audio|Components|Audio|Play (Variables|Default|GetAudio) 0.0)
  (if (== (Variables|Default|GetOwnCharacter) (Game|GetPlayerCharacter 0))
    ;[1 1 1] 데미지 요청 처리
    (CallFunction|ReqShoot (Transformation|GetActorLocation _returnvalue) (Transformation|GetActorForwardVector _returnvalue))))

(fn ConstructionScript)